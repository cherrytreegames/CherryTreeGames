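; First-person player character Blueprint handling movement, mouse and controller look, timeline-driven crouch, and a collision-free flying GodMode toggle.
; Pickup line-traces from the camera, sending tagged narrative items to the inventory or carrying objects with a PhysicsHandle whose target follows mouse look.
; Movement input checks velocity to start or clear a looping footstep-sound timer.
; Inventory and pause menu inputs manage their widgets, cursor and input mode.
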(event `self.ReceiveBeginPlay`
  ;[1 1 1] Inventory
  (bind _asfp_player_controller (cast `/Game/General/Character/FP_PlayerController` (`GameplayStatics.GetPlayerController` 0)))
  (set `self.PlayerControllerREF` _asfp_player_controller)
  (bind _returnvalue (`|CreateWidget` "/Game/General/UX/InventoryHUD/InventoryWidget_BP.InventoryWidget_BP_C"))
  (set `self.Inventory REF` _returnvalue))

(event `Footsteps Play`
  ;[1 1 1] Footstep Audio (Sorry about the mess guys XD)
  (`GameplayStatics.PlaySoundAtLocation` "/Game/General/Audio/A_Footsteps_v01_G_Cue.A_Footsteps_v01_G_Cue" (- (`self.K2_GetActorLocation`) (0.0 0.0 44.0)) (struct) 1.0 1.0 0.0 null null null))

(event `InputAction|Inventory`
  (params (Key :type "Key Structure"))
  (bind _inventory_ref (`self.Inventory REF`))
  ;[1 1 1] Inventory
  (:`Pressed`
    (`/Engine/EditorBlueprintResources/StandardMacros.IsValid` (`self.Inventory REF`)
      (:`Is Valid`
        _)
      (:`Is Not Valid`
        (bind _returnvalue (`|CreateWidget` "/Game/General/UX/InventoryHUD/InventoryWidget_BP.InventoryWidget_BP_C"))
        (set `self.Inventory REF` _returnvalue)))
    (`/Engine/EditorBlueprintResources/StandardMacros.FlipFlop`
      (:`A`
        (`WidgetBlueprintLibrary.SetInputMode_GameAndUIEx` (`self.PlayerControllerREF`) (`self.HUD_REF`))
        (set `PlayerController.bShowMouseCursor` true (`self.PlayerControllerREF`))
        (`UserWidget.AddToViewport` _inventory_ref 0))
      (:`B`
        (set `PlayerController.bShowMouseCursor` false (`self.PlayerControllerREF`))
        (`WidgetBlueprintLibrary.SetInputMode_GameOnly` (`self.PlayerControllerREF`))
        (`Widget.RemoveFromParent` _inventory_ref)))))

(event `InputAxis|LookXController`
  (params (AxisValue :type "Float (single-precision)"))
  ;[1 1 1] Controller Look
  (`self.AddControllerYawInput` (* AxisValue (`self.ContrrollerXRate`) (`GameplayStatics.GetWorldDeltaSeconds`))))

(event `InputAction|Pause`
  (params (Key :type "Key Structure"))
  (bind _returnvalue (`GameplayStatics.GetPlayerController` 0))
  (bind _pausemenuref (`self.PauseMenuREF`))
  ;[1 1 1] Pause Menu
  (:`Pressed`
    (`/Engine/EditorBlueprintResources/StandardMacros.IsValid` (`self.PauseMenuREF`)
      (:`Is Valid`
        _)
      (:`Is Not Valid`
        (bind _returnvalue_2 (`|CreateWidget` "/Game/General/UX/PauseMenu/M_PauseMenuWidget_v01_G.M_PauseMenuWidget_v01_G_C"))
        (set `self.PauseMenuREF` _returnvalue_2)))
    (if (`GameplayStatics.IsGamePaused`)
      (`Widget.RemoveFromParent` _pausemenuref)
      (bind _returnvalue_3 (`GameplayStatics.SetGamePaused` false))
      (set `PlayerController.bShowMouseCursor` _returnvalue_3 _returnvalue)
      (`WidgetBlueprintLibrary.SetInputMode_GameOnly` _returnvalue)
      (else
        (`UserWidget.AddToViewport` _pausemenuref 0)
        (`GameplayStatics.SetGamePaused` false)
        (set `PlayerController.bShowMouseCursor` true _returnvalue)
        (`WidgetBlueprintLibrary.SetInputMode_GameAndUIEx` _returnvalue _pausemenuref "LockInFullscreen" false)))))

(event `InputAxis|Forward/Back`
  (params (AxisValue :type "Float (single-precision)"))
  (bind (_returnvalue_x _returnvalue_y _returnvalue_z) (`KismetMathLibrary.BreakVector` (`self.GetVelocity`)))
  ;[1 1 1] Movement
  (`self.AddMovementInput` (`KismetMathLibrary.GetForwardVector` (`KismetMathLibrary.MakeRotator` 0.0 0.0 (.yaw (`self.GetControlRotation`)))) AxisValue)
  ;[1 1 1] Footstep Audio (Sorry about the mess guys XD)
  (if (and (or (> _returnvalue_x 2.0) (< _returnvalue_x -20.0) (> _returnvalue_y 2.0) (< _returnvalue_y -20.0)) (== _returnvalue_z 0.0)) :!label _label
    (`/Engine/EditorBlueprintResources/StandardMacros.DoOnce` false :!label _label_2
      (:`Completed`
        (bind _returnvalue (`KismetSystemLibrary.K2_SetTimerDelegate` (delegate `Footsteps Play`) (`self.FootstepInterval`) true))))
    (else
      (`KismetSystemLibrary.K2_ClearAndInvalidateTimerHandle` _returnvalue)
      (goto _label_2 :!via `Reset`))))

(event `InputAxis|LookYController`
  (params (AxisValue :type "Float (single-precision)"))
  ;[1 1 1] Controller Look
  (`self.AddControllerPitchInput` (* AxisValue (`self.ControllerYRate`) (`GameplayStatics.GetWorldDeltaSeconds`))))

(event `InputAxis|Right/Left`
  (params (AxisValue :type "Float (single-precision)"))
  ;[1 1 1] Movement
  (`self.AddMovementInput` (`KismetMathLibrary.GetRightVector` (`KismetMathLibrary.MakeRotator` 0.0 0.0 (.yaw (`self.GetControlRotation`)))) AxisValue)
  (goto _label))

(event `InputAxis|MouseY`
  (params (AxisValue :type "Float (single-precision)"))
  (bind _fp_camera (`self.FP_Camera`))
  ;[1 1 1] Looking
  (`self.AddControllerPitchInput` AxisValue)
  (`PhysicsHandleComponent.SetTargetLocation` (`self.PhysicsHandle`) (+ (* (`SceneComponent.GetForwardVector` _fp_camera) 200.0) (`SceneComponent.K2_GetComponentLocation` _fp_camera))))

(event `OverlappedKeypad`
  (params (`Current Actor` :type "Actor Object Reference"))
  (set `self.CurrentKeypadActor` `Current Actor`))

(event `InputAction|Crouch`
  (params (Key :type "Key Structure"))
  ;[1 1 1] Crouch
  (:`Pressed`
    (bind (_direction _capsuleheight) (`Timeline|Timeline_0` :!label _label_3)
      (:`Update`
        (`CapsuleComponent.SetCapsuleHalfHeight` (`self.CapsuleComponent`) _capsuleheight true))))
  (:`Released`
    (goto _label_3 :!via `Reverse`)))

(event `InputAxis|MouseX`
  (params (AxisValue :type "Float (single-precision)"))
  (bind _fp_camera (`self.FP_Camera`))
  ;[1 1 1] Looking
  (`self.AddControllerYawInput` AxisValue)
  (`PhysicsHandleComponent.SetTargetLocation` (`self.PhysicsHandle`) (+ (* (`SceneComponent.GetForwardVector` _fp_camera) 200.0) (`SceneComponent.K2_GetComponentLocation` _fp_camera))))

(event `InputAction|GodMode`
  (params (Key :type "Key Structure"))
  (bind _charactermovement (`self.CharacterMovement`))
  ;[1 1 1] NoClip/Fly Note:Flying doesn't have horizontal motion, I don't know why.
  (:`Pressed`
    (bind _output_get (set `self.GodMode` (not (`self.GodMode`))))
    (if _output_get
      (`self.SetActorEnableCollision` false)
      (`CharacterMovementComponent.SetMovementMode` _charactermovement "MOVE_Flying" 0)
      (else
        (`self.SetActorEnableCollision` true)
        (`CharacterMovementComponent.SetMovementMode` _charactermovement "MOVE_Walking" 0)))))

(event `InputAction|Pickup`
  (params (Key :type "Key Structure"))
  (bind _fp_camera (`self.FP_Camera`))
  (bind _returnvalue (`SceneComponent.K2_GetComponentLocation` _fp_camera))
  ;[1 1 1] Pickup
  (:`Pressed`
    (if (`self.HoldingItem`)
      (`PhysicsHandleComponent.ReleaseComponent` (`self.PhysicsHandle`))
      (set `self.HoldingItem` false)
      (else
        (bind (_outhit _returnvalue_2) (`KismetSystemLibrary.LineTraceSingle` _returnvalue (+ (* (`SceneComponent.GetForwardVector` _fp_camera) 200.0) _returnvalue) "TraceTypeQuery1"))
        (if _returnvalue_2
          (bind (_bblockinghit _binitialoverlap _time _distance _location _impactpoint _normal _impactnormal _physmat _hitactor _hitcomponent) (`GameplayStatics.BreakHitResult` _outhit))
          (if (`self.ActorHasTag` _hitactor (`self.NarrativeTag`))
            (`/Game/General/UX/InventoryHUD/InventoryWidget_BP.Item1` (`self.Inventory REF`))
            (`self.K2_DestroyActor` _hitactor)
            (else
              (`PhysicsHandleComponent.GrabComponentAtLocationWithRotation` :`self` (`self.PhysicsHandle`) :`Component` _hitcomponent :`Location` (`SceneComponent.K2_GetComponentLocation` _hitcomponent))
              (set `self.HoldingItem` (`KismetSystemLibrary.IsValid` _hitactor)))))))))

(fn `CrouchAnim`
  (params (bState :type Boolean))
  (if bState
    _))

(fn `UserConstructionScript`)