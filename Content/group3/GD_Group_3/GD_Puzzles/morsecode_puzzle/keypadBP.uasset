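; Keypad-locked safe that opens its door when the player enters the correct code.
; A trigger box enables input and registers the keypad with FP_PlayerBP, and Interact opens KeypadUI with the game paused.
; ConfirmCode compares the code to NeededCode, playing a locked sound or setting Success, animating handle then door via timelines, and clearing the player's safe objective.
; Cursor hover toggles a material parameter on the keypad mesh.
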(event `InputAction|Interact`
  (params (Key :type "Key Structure"))
  (bind _returnvalue (`GameplayStatics.GetPlayerController` 0))
  (:`Pressed`
    (bind _returnvalue_2 (`|CreateWidget` "/Game/group3/GD_Group_3/GD_Puzzles/morsecode_puzzle/KeypadUI.KeypadUI_C"))
    (`UserWidget.AddToViewport` _returnvalue_2 0)
    (set `PlayerController.bShowMouseCursor` true _returnvalue)
    (`GameplayStatics.SetGamePaused` true)
    (`WidgetBlueprintLibrary.SetInputMode_UIOnlyEx` _returnvalue null)))

(event `ConfirmCode`
  (params (`Code To Confirm` :type String))
  (if (`KismetStringLibrary.EqualEqual_StrStr` (`self.NeededCode`) `Code To Confirm`)
    (set `self.Success` true)
    (`GameplayStatics.PlaySoundAtLocation` "/Game/General/Audio/A_MenuPing_v01_G_Cue.A_MenuPing_v01_G_Cue" (0.0 0.0 0.0) (struct) 1.0 1.0 0.0 null null null)
    (`GameplayStatics.PlaySoundAtLocation` "/Game/group3/Audio_Group_3/A_MetalDoorHandle_v01_S_Cue.A_MetalDoorHandle_v01_S_Cue" (0.0 0.0 0.0) (struct) 1.0 1.0 0.0 null null null)
    (bind (_direction _handleanim) (`Timeline|HandleAnim`)
      (:`Update`
        (`SceneComponent.K2_SetRelativeRotation` (`self.HandleRotator`) (`KismetMathLibrary.MakeRotator` 0.0 _handleanim) false false)
        (`KismetSystemLibrary.Delay` 1.0)
        (bind (_direction_2 _dooranim) (`Timeline|DoorAnim`)
          (:`Update`
            (`SceneComponent.K2_SetRelativeRotation` (`self.RotatePoint`) (`KismetMathLibrary.MakeRotator` 0.0 0.0 _dooranim) false false)
            (bind _asfp_player_bp (cast `/Game/General/Character/FP_PlayerBP` (stale `self.Box.OnComponentBeginOverlap` OtherActor)))
            (bind _output_get (set `self.Objective` "Find a way into the safe"))
            (if (`KismetStringLibrary.EqualEqual_StrStr` (`/Game/General/Character/FP_PlayerBP.Current Objective` _asfp_player_bp) _output_get)
              (`/Game/General/Character/FP_PlayerBP.Slide Off` _asfp_player_bp)
              (set `/Game/General/Character/FP_PlayerBP.Current Objective` "" _asfp_player_bp)
              (`GameplayStatics.PlaySound2D` "/Game/General/Audio/A_Notification_v01_G.A_Notification_v01_G" 1.0 1.0 0.0 null null)))))
      (:`Finished`
        (`GameplayStatics.PlaySoundAtLocation` "/Game/group3/Audio_Group_3/A_Safedoor_v01_S_Cue.A_Safedoor_v01_S_Cue" (0.0 0.0 0.0) (struct) 1.0 1.0 0.0 null null null)))
    (else
      (`GameplayStatics.PlaySoundAtLocation` "/Game/group3/Audio_Group_3/A_LockedDoor_v01_S_Cue.A_LockedDoor_v01_S_Cue" (0.0 0.0 0.0) (struct) 1.0 1.0 0.0 null null null))))

(event `self.Box.OnComponentBeginOverlap`
  (params (OverlappedComponent :type "PrimitiveComponent Object Reference") (OtherActor :type "Actor Object Reference") (OtherComp :type "PrimitiveComponent Object Reference") (OtherBodyIndex :type Integer) (bFromSweep :type Boolean) (SweepResult :type "HitResult Structure (by ref)"))
  (bind _asfp_player_bp (cast `/Game/General/Character/FP_PlayerBP` OtherActor))
  (`self.EnableInput` (`GameplayStatics.GetPlayerController` 0))
  (`/Game/General/Character/FP_PlayerBP.OverlappedKeypad` _asfp_player_bp self))

(event `self.Box.OnComponentEndOverlap`
  (params (OverlappedComponent :type "PrimitiveComponent Object Reference") (OtherActor :type "Actor Object Reference") (OtherComp :type "PrimitiveComponent Object Reference") (OtherBodyIndex :type Integer))
  (cast `/Game/General/Character/FP_PlayerBP` OtherActor)
  (`self.DisableInput` (`GameplayStatics.GetPlayerController` 0)))

(event `self.KeypadMesh.OnBeginCursorOver`
  (params (TouchedComponent :type "PrimitiveComponent Object Reference"))
  (`MeshComponent.SetScalarParameterValueOnMaterials` (`self.KeypadMesh`) "B_1" 1.0))

(event `self.KeypadMesh.OnEndCursorOver`
  (params (TouchedComponent :type "PrimitiveComponent Object Reference"))
  (`MeshComponent.SetScalarParameterValueOnMaterials` (`self.KeypadMesh`) "B_1" 0.0))

(fn `CheckSuccess`
  (returns (Success :type Boolean))
  (return (`self.Success`)))

(fn `UserConstructionScript`)