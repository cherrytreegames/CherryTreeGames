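; Pressure plate puzzle button that switches a linked object through TurnSwitchMessage.
; Beginning an overlap on the trigger plays a sound and, if unpressed, runs the PushDown timeline to move the plate vertically.
; Ending an overlap replays the sound and reverses the timeline only if the trigger's overlapping-actor list still has an entry.
; When the timeline finishes either way, it swaps the plate material and sends the pressed state to ObjectAffected.
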(event `self.Trigger.OnComponentBeginOverlap`
  (params (OverlappedComponent :type "PrimitiveComponent Object Reference") (OtherActor :type "Actor Object Reference") (OtherComp :type "PrimitiveComponent Object Reference") (OtherBodyIndex :type Integer) (bFromSweep :type Boolean) (SweepResult :type "HitResult Structure (by ref)"))
  (`GameplayStatics.PlaySoundAtLocation` "/Game/group3/Audio_Group_3/A_PresurePlate_v01_S_Cue.A_PresurePlate_v01_S_Cue" (0.0 0.0 0.0) (struct) 1.0 1.0 0.0 null null null)
  (if (not (`self.Pressed`))
    (set `self.Pressed` true)
    (bind (_direction _newtrack_0) (`Timeline|PushDown` :!label _label)
      (:`Update`
        (`SceneComponent.K2_SetRelativeLocation` (`self.Plate`) (`KismetMathLibrary.MakeVector` 0.0 0.0 _newtrack_0) false false))
      (:`Finished`
        (if (`self.Pressed`)
          (`PrimitiveComponent.SetMaterial` (`self.Plate`) 0 "/Game/group3/Props_Group_3/PressurePlate2/Triggered/M_PressurePlateNotTriggered_V01_S.M_PressurePlateNotTriggered_V01_S")
          (else
            (`PrimitiveComponent.SetMaterial` (`self.Plate`) 0 "/Game/group3/Props_Group_3/PressurePlate2/NotTriggered/M_PressurePlateTop_V01_S.M_PressurePlateTop_V01_S")))
        (message `/Game/group3/GD_Group_3/GD_Puzzles/pressureplate_puzzle/TurnSwitchBP.TurnSwitch` (`self.ObjectAffected`) (`self.Pressed`))))))

(event `self.Trigger.OnComponentEndOverlap`
  (params (OverlappedComponent :type "PrimitiveComponent Object Reference") (OtherActor :type "Actor Object Reference") (OtherComp :type "PrimitiveComponent Object Reference") (OtherBodyIndex :type Integer))
  (`GameplayStatics.PlaySoundAtLocation` "/Game/group3/Audio_Group_3/A_PresurePlate_v01_S_Cue.A_PresurePlate_v01_S_Cue" (0.0 0.0 0.0) (struct) 1.0 1.0 0.0 null null null)
  (if (`KismetArrayLibrary.Array_IsValidIndex` (`PrimitiveComponent.GetOverlappingActors` (`self.Trigger`) null))
    (set `self.Pressed` false)
    (goto _label :!via `Reverse`)))

(fn `UserConstructionScript`)