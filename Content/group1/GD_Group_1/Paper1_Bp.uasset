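; Paper1_Bp is an interactable paper actor that the player can remove from the level when nearby.
; Its widget component is hidden at BeginPlay, shown when an actor begins overlapping the sphere, and hidden again on end overlap.
; The overlap events also enable and disable input for player 0.
; Pressing Interact destroys the paper if the actor from the begin overlap event casts to Character.
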(event `self.ReceiveBeginPlay`
  (`SceneComponent.SetVisibility` (`self.WidgetComponent`) false false))

(event `self.SphereComponent.OnComponentBeginOverlap`
  (params (OverlappedComponent :type "PrimitiveComponent Object Reference") (OtherActor :type "Actor Object Reference") (OtherComp :type "PrimitiveComponent Object Reference") (OtherBodyIndex :type Integer) (bFromSweep :type Boolean) (SweepResult :type "HitResult Structure (by ref)"))
  (`SceneComponent.SetVisibility` (`self.WidgetComponent`) true false)
  (`self.EnableInput` (`GameplayStatics.GetPlayerController` 0)))

(event `self.SphereComponent.OnComponentEndOverlap`
  (params (OverlappedComponent :type "PrimitiveComponent Object Reference") (OtherActor :type "Actor Object Reference") (OtherComp :type "PrimitiveComponent Object Reference") (OtherBodyIndex :type Integer))
  (`SceneComponent.SetVisibility` (`self.WidgetComponent`) false false)
  (`self.DisableInput` (`GameplayStatics.GetPlayerController` 0)))

(event `InputAction|Interact`
  (params (Key :type "Key Structure"))
  (:`Pressed`
    (cast `Character` (stale `self.SphereComponent.OnComponentBeginOverlap` OtherActor))
    (`self.K2_DestroyActor`)))

(fn `UserConstructionScript`)