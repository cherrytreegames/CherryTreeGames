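; VentCover_BP is an interactable vent cover with four screws that the player turns with a screwdriver.
; Its sphere trigger toggles input and an interaction prompt; Interact opens VentWidget_BP and shows the mouse cursor.
; SetActiveButton picks the active screw, and each mouse wheel-up plays a timeline that rotates it and the screwdriver, flipping the screwdriver's pitch step based on its current rotation.
; No unscrew completion or cover removal is handled here.
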(event `self.ReceiveBeginPlay`
  (`SceneComponent.SetVisibility` (`self.InteractionWidget`) false false)
  (set `self.ScrewsArray` (`|MakeArray` (`self.ScrewRoot1`) (`self.ScrewRoot2`) (`self.ScrewRoot3`) (`self.ScrewRoot4`))))

(event `self.SphereComponent.OnComponentBeginOverlap`
  (params (OverlappedComponent :type "PrimitiveComponent Object Reference") (OtherActor :type "Actor Object Reference") (OtherComp :type "PrimitiveComponent Object Reference") (OtherBodyIndex :type Integer) (bFromSweep :type Boolean) (SweepResult :type "HitResult Structure (by ref)"))
  (`self.EnableInput` (`GameplayStatics.GetPlayerController` 0))
  (`SceneComponent.SetVisibility` (`self.InteractionWidget`) true false))

(event `self.SphereComponent.OnComponentEndOverlap`
  (params (OverlappedComponent :type "PrimitiveComponent Object Reference") (OtherActor :type "Actor Object Reference") (OtherComp :type "PrimitiveComponent Object Reference") (OtherBodyIndex :type Integer))
  (`self.DisableInput` (`GameplayStatics.GetPlayerController` 0))
  (`SceneComponent.SetVisibility` (`self.InteractionWidget`) false false))

(event `InputAction|Interact`
  (params (Key :type "Key Structure"))
  (bind _returnvalue (`GameplayStatics.GetPlayerController` 0))
  (:`Pressed`
    (`SceneComponent.SetVisibility` (`self.InteractionWidget`) false false)
    (bind _returnvalue_2 (`|CreateWidget` "/Game/group1/GD_Group_1/Widgets/VentWidget_BP.VentWidget_BP_C" _returnvalue))
    (`UserWidget.AddToViewport` _returnvalue_2 0)
    (set `PlayerController.bShowMouseCursor` true _returnvalue)))

(event `Key|MouseScrollUp`
  (params (Key :type "Key Structure"))
  (bind _screwdriver (`self.Screwdriver`))
  (bind (_relativerotation_roll _relativerotation_pitch _relativerotation_yaw) (`KismetMathLibrary.BreakRotator` (`SceneComponent.RelativeRotation` (`self.Screwdriver`))))
  (:`Pressed`
    (bind (_direction _newtrack_0) (`Timeline|ScrewerAnimation` :!via `PlayFromStart`)
      (:`Update`
        (if (or (> _relativerotation_yaw -90.0) (> _relativerotation_pitch 90.0))
          (bind _returnvalue (`KismetMathLibrary.MakeRotator` 0.0 _newtrack_0))
          (`SceneComponent.K2_AddRelativeRotation` _screwdriver _returnvalue false false)
          (else
            (`SceneComponent.K2_AddRelativeRotation` _screwdriver (`KismetMathLibrary.MakeRotator` 0.0 (* -1 _newtrack_0)) false false)))
        (`SceneComponent.K2_AddRelativeRotation` (`|GetArrayItem` (`self.ScrewsArray`) (`self.ActiveIndex`)) _returnvalue false false)))))

(fn `Set Active Button`
  (params (Digit :type Integer))
  (set `self.ActiveIndex` Digit))

(fn `UserConstructionScript`)