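; Toy prop in the computer puzzle group that makes impact sounds and completes the left-click pickup tutorial objective.
; Hits play a sound at the impact point, with volume from the mesh's X velocity, clamped and throttled by a delayed DoOnce reset.
; Clicking it during that objective calls SlideOff on FP_PlayerBP, clears the objective and plays a notification.
; Cursor hover toggles the B_1 material parameter on the mesh.
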(event `self.ReceiveHit`
  (params (MyComp :type "PrimitiveComponent Object Reference") (Other :type "Actor Object Reference") (OtherComp :type "PrimitiveComponent Object Reference") (bSelfMoved :type Boolean) (HitLocation :type "Vector Structure") (HitNormal :type "Vector Structure") (NormalImpulse :type "Vector Structure") (Hit :type "HitResult Structure (by ref)"))
  (`/Engine/EditorBlueprintResources/StandardMacros.DoOnce` false :!label _label
    (:`Completed`
      (`GameplayStatics.PlaySoundAtLocation` "/Game/General/Audio/A_Toy_v01_G_Cue.A_Toy_v01_G_Cue" HitLocation (struct) (`KismetMathLibrary.FClamp` (`KismetMathLibrary.SafeDivide` (`KismetMathLibrary.VSize` (`KismetMathLibrary.Conv_DoubleToVector` (.x (`SceneComponent.GetComponentVelocity` (`self.StaticMesh`))))) 1200.0) 0.0 0.7) 1.0 0.0 null null null)
      (`KismetSystemLibrary.Delay` 0.38)
      (goto _label :!via `Reset`))))

(event `self.ReceiveActorOnClicked`
  (params (ButtonPressed :type "Key Structure"))
  ;[1 1 1] complete objective
  (bind _asfp_player_bp (cast `/Game/General/Character/FP_PlayerBP` (`GameplayStatics.GetPlayerCharacter` 0)))
  (if (`KismetStringLibrary.EqualEqual_StrStr` (`/Game/General/Character/FP_PlayerBP.Current Objective` _asfp_player_bp) "Use Left Click to pick up items")
    (`/Game/General/Character/FP_PlayerBP.Slide Off` _asfp_player_bp)
    (set `/Game/General/Character/FP_PlayerBP.Current Objective` "" _asfp_player_bp)
    (`GameplayStatics.PlaySound2D` "/Game/General/Audio/A_Notification_v01_G.A_Notification_v01_G" 1.0 1.0 0.0 null null)))

(event `self.StaticMesh.OnBeginCursorOver`
  (params (TouchedComponent :type "PrimitiveComponent Object Reference"))
  (`MeshComponent.SetScalarParameterValueOnMaterials` (`self.StaticMesh`) "B_1" 1.0))

(event `self.StaticMesh.OnEndCursorOver`
  (params (TouchedComponent :type "PrimitiveComponent Object Reference"))
  (`MeshComponent.SetScalarParameterValueOnMaterials` (`self.StaticMesh`) "B_1" 0.0))

(fn `UserConstructionScript`)