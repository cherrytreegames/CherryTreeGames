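; FileBox_BP is an interactable box in the EmergencyBox folder that the player can open once.
; Overlapping its sphere while closed shows a prompt widget and enables player input; leaving hides it and disables input.
; Interact sets IsOpen, hides the widget and plays a timeline that adds its track value as relative yaw to Root each update, so rotation accumulates.
; Disconnected nodes targeting Map_BP never run.
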(event `self.ReceiveBeginPlay`
  (`SceneComponent.SetVisibility` (`self.Widget`) false false))

(event `self.Sphere.OnComponentBeginOverlap`
  (params (OverlappedComponent :type "PrimitiveComponent Object Reference") (OtherActor :type "Actor Object Reference") (OtherComp :type "PrimitiveComponent Object Reference") (OtherBodyIndex :type Integer) (bFromSweep :type Boolean) (SweepResult :type "HitResult Structure (by ref)"))
  (if (not (`self.IsOpen`))
    (`SceneComponent.SetVisibility` (`self.Widget`) true false)
    (`self.EnableInput` (`GameplayStatics.GetPlayerController` 0))))

(event `self.Sphere.OnComponentEndOverlap`
  (params (OverlappedComponent :type "PrimitiveComponent Object Reference") (OtherActor :type "Actor Object Reference") (OtherComp :type "PrimitiveComponent Object Reference") (OtherBodyIndex :type Integer))
  (`SceneComponent.SetVisibility` (`self.Widget`) false false)
  (`self.DisableInput` (`GameplayStatics.GetPlayerController` 0)))

(event `InputAction|Interact`
  (params (Key :type "Key Structure"))
  (:`Pressed`
    (if (not (`self.IsOpen`))
      (`SceneComponent.SetVisibility` (`self.Widget`) false false)
      (set `self.IsOpen` true)
      (bind (_direction _newtrack_0) (`Timeline|Timeline_0`)
        (:`Update`
          (`SceneComponent.K2_AddRelativeRotation` (`self.Root`) (`KismetMathLibrary.MakeRotator` 0.0 0.0 _newtrack_0) false false))))))

(fn `UserConstructionScript`)