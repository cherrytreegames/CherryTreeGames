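; Breakable emergency box actor that gives the player a key when its destructible component fractures.
; On fracture it sets HasKey on the player's FP_PlayerBP and shows a KeyCollection_BP widget.
; After short delays it destroys the first EKey_BP found in the level, then removes the widget from the viewport.
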(event `self.Destructible.OnComponentFracture`
  (params (HitPoint :type "Vector Structure (by ref)") (HitDirection :type "Vector Structure (by ref)"))
  (bind _asfp_player_bp (cast `/Game/General/Character/FP_PlayerBP` (`GameplayStatics.GetPlayerCharacter` 0)))
  (set `/Game/General/Character/FP_PlayerBP.HasKey` true _asfp_player_bp)
  (bind _returnvalue (`|CreateWidget` "/Game/group1/GD_Group_1/Widgets/KeyCollection_BP.KeyCollection_BP_C" (`GameplayStatics.GetPlayerController` 0)))
  (`UserWidget.AddToViewport` _returnvalue 0)
  (bind _outactors (`GameplayStatics.GetAllActorsOfClass` "/Game/group1/GD_Group_1/EmergencyBox/EKey_BP.EKey_BP_C"))
  (`KismetSystemLibrary.Delay` 0.5)
  (`self.K2_DestroyActor` (`|GetArrayItem` _outactors))
  (`KismetSystemLibrary.Delay` 2.0)
  (`Widget.RemoveFromParent` _returnvalue))

(fn `UserConstructionScript`)