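; Map_BP is a pickup actor for a map, granted to the player on interaction.
; A sphere overlap shows a prompt widget while IsOpen is true, and leaving the sphere hides it.
; Pressing Interact while open calls Item5 on a newly created inventory widget, shows a collection widget for two seconds, then destroys the actor.
; The Interact handler checks only IsOpen, not whether the player overlaps the sphere.
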(event `self.ReceiveBeginPlay`
  (`SceneComponent.SetVisibility` (`self.Widget`) false false))

(event `self.Sphere.OnComponentBeginOverlap`
  (params (OverlappedComponent :type "PrimitiveComponent Object Reference") (OtherActor :type "Actor Object Reference") (OtherComp :type "PrimitiveComponent Object Reference") (OtherBodyIndex :type Integer) (bFromSweep :type Boolean) (SweepResult :type "HitResult Structure (by ref)"))
  (if (`self.IsOpen`)
    (`SceneComponent.SetVisibility` (`self.Widget`) true false)))

(event `self.Sphere.OnComponentEndOverlap`
  (params (OverlappedComponent :type "PrimitiveComponent Object Reference") (OtherActor :type "Actor Object Reference") (OtherComp :type "PrimitiveComponent Object Reference") (OtherBodyIndex :type Integer))
  (`SceneComponent.SetVisibility` (`self.Widget`) false false))

(event `InputAction|Interact`
  (params (Key :type "Key Structure"))
  (:`Pressed`
    (if (`self.IsOpen`)
      (`SceneComponent.SetVisibility` (`self.Widget`) false false)
      (bind _returnvalue (`|CreateWidget` "/Game/General/UX/InventoryHUD/InventoryWidget_BP.InventoryWidget_BP_C" (`GameplayStatics.GetPlayerController` 0)))
      (`/Game/General/UX/InventoryHUD/InventoryWidget_BP.Item5` _returnvalue)
      (bind _returnvalue_2 (`|CreateWidget` "/Game/group1/GD_Group_1/Widgets/MapCollection_BP.MapCollection_BP_C"))
      (`UserWidget.AddToViewport` _returnvalue_2 0)
      (`KismetSystemLibrary.Delay` 2.0)
      (`Widget.RemoveFromParent` _returnvalue_2)
      (`self.K2_DestroyActor`))))

(fn `UserConstructionScript`)