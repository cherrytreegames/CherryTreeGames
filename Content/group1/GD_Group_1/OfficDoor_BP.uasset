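; OfficDoor_BP is an interactable office door that the player opens once with the Interact input.
; Overlapping its box component while closed shows a widget prompt and enables input, and leaving hides the prompt and disables input.
; Interact hides the prompt and plays the DoorOpening timeline, which cumulatively adds its track value to the Rotator's yaw each update, then sets IsOpen on finish.
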(event `self.ReceiveBeginPlay`
  (`SceneComponent.SetVisibility` (`self.WidgetCompoent`) false false))

(event `self.BoxComponent.OnComponentBeginOverlap`
  (params (OverlappedComponent :type "PrimitiveComponent Object Reference") (OtherActor :type "Actor Object Reference") (OtherComp :type "PrimitiveComponent Object Reference") (OtherBodyIndex :type Integer) (bFromSweep :type Boolean) (SweepResult :type "HitResult Structure (by ref)"))
  (if (not (`self.IsOpen`))
    (`SceneComponent.SetVisibility` (`self.WidgetCompoent`) true false)
    (`self.EnableInput` (`GameplayStatics.GetPlayerController` 0))))

(event `self.BoxComponent.OnComponentEndOverlap`
  (params (OverlappedComponent :type "PrimitiveComponent Object Reference") (OtherActor :type "Actor Object Reference") (OtherComp :type "PrimitiveComponent Object Reference") (OtherBodyIndex :type Integer))
  (`SceneComponent.SetVisibility` (`self.WidgetCompoent`) false false)
  (`self.DisableInput` (`GameplayStatics.GetPlayerController` 0)))

(event `InputAction|Interact`
  (params (Key :type "Key Structure"))
  (:`Pressed`
    (`SceneComponent.SetVisibility` (`self.WidgetCompoent`) false false)
    (if (not (`self.IsOpen`))
      (bind (_direction _dooropeningtrack) (`Timeline|DoorOpening`)
        (:`Update`
          (`SceneComponent.K2_AddRelativeRotation` (`self.Rotator`) (`KismetMathLibrary.MakeRotator` 0.0 0.0 _dooropeningtrack) false false))
        (:`Finished`
          (set `self.IsOpen` true))))))

(fn `UserConstructionScript`)