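; Scanner_BP is a keycard scanner that opens the hall door once it has been activated.
; Its screen starts red at BeginPlay, and the Activate function sets IsActivated and switches the screen to a green material.
; When a Keycard_BP overlaps the trigger while activated, it calls OpenDoor on the first HallDoor_BP found in the level.
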(event `self.ReceiveBeginPlay`
  (`PrimitiveComponent.SetMaterial` (`self.ColorScreen`) 0 (`self.RedMat`)))

(event `self.Trigger.OnComponentBeginOverlap`
  (params (OverlappedComponent :type "PrimitiveComponent Object Reference") (OtherActor :type "Actor Object Reference") (OtherComp :type "PrimitiveComponent Object Reference") (OtherBodyIndex :type Integer) (bFromSweep :type Boolean) (SweepResult :type "HitResult Structure (by ref)"))
  (cast `/Game/group1/GD_Group_1/Keycard_BP` OtherActor)
  (if (`self.IsActivated`)
    (bind _outactors (`GameplayStatics.GetAllActorsOfClass` "/Game/group1/GD_Group_1/ComputerPuzzle/HallDoor_BP.HallDoor_BP_C"))
    (`/Game/group1/GD_Group_1/ComputerPuzzle/HallDoor_BP.OpenDoor` (`|GetArrayItem` _outactors))))

(fn `Activate`
  (set `self.IsActivated` true)
  (`PrimitiveComponent.SetMaterial` (`self.ColorScreen`) 0 (`self.GreenMat`)))

(fn `UserConstructionScript`)