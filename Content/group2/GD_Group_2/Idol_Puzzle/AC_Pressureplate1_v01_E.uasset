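; Pressure plate for an idol puzzle that accepts two specific idol actors placed on it.
; Each collision component casts the overlapping actor to its matching idol class and sets that idol's placed flag.
; A DoOnce then assigns the idol's mesh to the plate's static mesh component and destroys the incoming actor, so the idol appears seated in place.
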(event `self.Collision4idol1.OnComponentBeginOverlap`
  (params (OverlappedComponent :type "PrimitiveComponent Object Reference") (OtherActor :type "Actor Object Reference") (OtherComp :type "PrimitiveComponent Object Reference") (OtherBodyIndex :type Integer) (bFromSweep :type Boolean) (SweepResult :type "HitResult Structure (by ref)"))
  (bind _asac_idol_1_v_01_e (cast `/Game/group2/GD_Group_2/Idol_Puzzle/AC_Idol1_v01_E` OtherActor))
  (set `self.Idolplaced1` true)
  (if (`self.Idolplaced1`)
    (`/Engine/EditorBlueprintResources/StandardMacros.DoOnce` false
      (:`Completed`
        (`StaticMeshComponent.SetStaticMesh` (`self.Idol1`) "/Game/group2/Props_Group_2/Idols/P_AnchIdol_v01_e.P_AnchIdol_v01_E")
        (`self.K2_DestroyActor` _asac_idol_1_v_01_e)))))

(event `self.Collision4idol2.OnComponentBeginOverlap`
  (params (OverlappedComponent :type "PrimitiveComponent Object Reference") (OtherActor :type "Actor Object Reference") (OtherComp :type "PrimitiveComponent Object Reference") (OtherBodyIndex :type Integer) (bFromSweep :type Boolean) (SweepResult :type "HitResult Structure (by ref)"))
  (bind _asac_idol_2_v_01_e (cast `/Game/group2/GD_Group_2/Idol_Puzzle/AC_Idol2_v01_E` OtherActor))
  (set `self.Idolplaced2` true)
  (if (`self.Idolplaced2`)
    (`/Engine/EditorBlueprintResources/StandardMacros.DoOnce` false
      (:`Completed`
        (`StaticMeshComponent.SetStaticMesh` (`self.Idol2`) "/Game/group2/Props_Group_2/Idols/P_PharohIdol_v01_E.P_PharohIdol_v01_E")
        (`self.K2_DestroyActor` _asac_idol_2_v_01_e)))))

(fn `UserConstructionScript`)