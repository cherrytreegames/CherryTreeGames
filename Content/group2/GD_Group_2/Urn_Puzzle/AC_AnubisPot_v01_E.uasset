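; Anubis urn actor for the urn puzzle that accepts the matching Anubis head.
; When an Anubis head actor overlaps the Sphere, it sets a flag and plays a placement sound.
; Tick polls that flag and, through a DoOnce, swaps the Head mesh to the Anubis head and destroys the overlapping actor.
; Cursor hover over Head toggles a material scalar parameter.
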(event `self.Sphere.OnComponentBeginOverlap`
  (params (OverlappedComponent :type "PrimitiveComponent Object Reference") (OtherActor :type "Actor Object Reference") (OtherComp :type "PrimitiveComponent Object Reference") (OtherBodyIndex :type Integer) (bFromSweep :type Boolean) (SweepResult :type "HitResult Structure (by ref)"))
  (bind _asac_anubis_head_v_01_e (cast `/Game/group2/GD_Group_2/Urn_Puzzle/AC_AnubisHead_v01_E` OtherActor))
  (set `self.Correcthead1` true)
  ;[1 1 1] Sound when head placed
  (`GameplayStatics.PlaySoundAtLocation` "/Game/group2/Audio_Group_2/A_PotPlace_v01_E.A_PotPlace_v01_E" (`self.K2_GetActorLocation`) (struct) 1.0 1.0 0.0 null null null))

(event `self.ReceiveTick`
  (params (DeltaSeconds :type "Float (single-precision)"))
  (if (`self.Correcthead1`)
    (`/Engine/EditorBlueprintResources/StandardMacros.DoOnce` false
      (:`Completed`
        (`StaticMeshComponent.SetStaticMesh` (`self.Head`) "/Game/group2/Props_Group_2/Urns/Anubis/P_Anubishead_v01_E.P_Anubishead_v01_E")
        (`self.K2_DestroyActor` (stale `self.Sphere.OnComponentBeginOverlap` _asac_anubis_head_v_01_e))))))

(event `self.Head.OnBeginCursorOver`
  (params (TouchedComponent :type "PrimitiveComponent Object Reference"))
  (`MeshComponent.SetScalarParameterValueOnMaterials` (`self.Head`) "B_1" 1.0))

(event `self.Head.OnEndCursorOver`
  (params (TouchedComponent :type "PrimitiveComponent Object Reference"))
  (`MeshComponent.SetScalarParameterValueOnMaterials` (`self.Head`) "B_1" 0.0))

(fn `UserConstructionScript`)